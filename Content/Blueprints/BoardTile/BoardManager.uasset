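; BoardManager runs a checkers match against an AI playing Black, spawning the board and its starting pieces.
; Tile selection events drive movement, captures, kinging and forced multi-jumps, then switch turns and check for a side without moves.
; The AI applies each candidate to an encoded board snapshot, adds one random reply from live-board moves, and keeps the best material score.
; Game end shows a victory/defeat widget.
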(event Custom|StartAITurn
  (if (Variables|Default|GetGameOver)
    (Class|GameModeBase|ReturntoMainMenuHost (Game|GetGameMode))
    (else
      (Variables|Default|SetbIsAITurn true)
      (Utilities|FlowControl|Delay 1.0)
      (CallFunction|RunAITurn))))

(event Custom|AI_ContinueForcedJump
  (bind _keys (Utilities|Map|Keys (Variables|Default|GetValidMoves)))
  (if (> (Utilities|Array|Length _keys) 0)
    (Default|Select (Utilities|Array|Get(acopy) _keys (Math|Random|RandomIntegerinRange 0 (- (Utilities|Array|Length _keys) 1))))
    (Utilities|FlowControl|Delay 1.0)
    (if (Variables|Default|GetForcedDoubleJump)
      (CallFunction|AIContinueForcedJump))))

(event Custom|EndGame
  (Variables|Default|SetGameOver true)
  (Development|PrintString (Variables|Default|GetWinnerText) true true "(R=1.000000,G=0.080673,B=0.000000,A=1.000000)")
  (CallFunction|ShowVictoryDefeatWidget (Variables|Default|GetPlayerWon)))

(event Custom|OnSelected
  (params (Tile :type Board%20Tile%20Object%20Reference))
  ;[1 1 1] Tile Selection Handling
  (if (Variables|Default|GetForcedDoubleJump)
    ;[1 1 1] Handle Forced Doublejump
    (if (Utilities|Map|Contains (Variables|Default|GetValidMoves) Tile)
      (Variables|Default|SetForcedDoubleJump false)
      (Default|CallOnTileSelected Tile)
      ;[1 1 1] Do Movement into Selected Tile
      (bind _shouldking (CallFunction|TileShouldKing Tile (Variables|Default|GetActiveSelection) :!label _label))
      (Default|SetState (Variables|Default|GetActiveSelection) "NewEnumerator2" false)
      (Default|SetState Tile (Variables|Default|GetActivePlayer) _shouldking)
      (if (!= (.Value (Utilities|Map|Find (Variables|Default|GetValidMoves) Tile)) 0)
        (Default|SetState (.Value (Utilities|Map|Find (Variables|Default|GetValidMoves) Tile)) "NewEnumerator2" false)
        ;[1 1 1] Check for Forced Doublejump
        (bind _moves (Default|GetValidHops Tile true))
        (if (> (Utilities|Map|Length _moves) 0)
          (Variables|Default|SetValidMoves _moves)
          (Variables|Default|SetForcedDoubleJump true)
          (Variables|Default|SetActiveSelection Tile)
          (Development|PrintString "Found  a forced doublejump")
          (else
            (Utilities|Map|Clear (Variables|Default|GetValidMoves) :!label _label_2)
            (Variables|Default|SetActiveSelection 0)
            (CallFunction|EndPlayerTurn)
            (Development|PrintString "end player turn")))
        (else
          (goto _label_2))))
    (else
      (Default|CallOnTileSelected Tile)
      (if (== (Variables|Default|GetActiveSelection) 0)
        (if (Utilities|Enum|Equal(Enum) (Variables|/Game/Blueprints/BoardTile/BoardTile.BoardTile_C|GetState Tile) (Variables|Default|GetActivePlayer))
          (bind _output_get (Variables|Default|SetActiveSelection Tile))
          (bind _moves_2 (Default|GetValidMoves _output_get true))
          (Variables|Default|SetValidMoves _moves_2)
          (else
            (Utilities|Map|Clear (Variables|Default|GetValidMoves))))
        (elif (Utilities|Map|Contains (Variables|Default|GetValidMoves) Tile)
          (goto _label)
          (else
            (Utilities|Map|Clear (Variables|Default|GetValidMoves))
            (Variables|Default|SetActiveSelection 0)))))))

(event EventBeginPlay
  (bind _tilecount (Variables|Default|GetTileCount))
  (bind _returnvalue (- _tilecount 1))
  ;[1 1 1] Build Board
  (for _index (range 0 _returnvalue)
    (for _index_2 (range 0 _returnvalue)
      (bind _coordinate (CallFunction|TileIndextoCoordinate _index))
      (bind _coordinate_2 (CallFunction|TileIndextoCoordinate _index_2))
      (if (== (Math|Integer|%(Integer) (+ _index_2 _index) 2) 0)
        (bind _returnvalue_2 (Game|SpawnActorfromClass "/Game/Blueprints/BoardTile/BoardTile.BoardTile_C" (Math|Transform|MakeRelativeTransform (Math|Conversions|ToTransform(Vector) (Math|Vector|MakeVector _coordinate _coordinate_2 0.0)) (Transformation|GetActorTransform)) "Undefined" 0 0))
        (Utilities|Set|Add (Variables|Default|GetTiles) _returnvalue_2)
        (Variables|/Game/Blueprints/BoardTile/BoardTile.BoardTile_C|SetRow _returnvalue_2 _index)
        (Variables|/Game/Blueprints/BoardTile/BoardTile.BoardTile_C|SetColumn _returnvalue_2 _index_2)
        (Default|SetTileColor _returnvalue_2 "NewEnumerator0")
        (switch int _index
          (:0
            (Default|SetState _returnvalue_2 "NewEnumerator1" false :!label _label)
            (EventDispatchers|BindEventtoOnSelected _returnvalue_2 (delegate Custom|OnSelected)))
          (:1
            (goto _label))
          (:2
            (goto _label))
          (:3
            (Default|SetState _returnvalue_2 "NewEnumerator2" false :!label _label_2)
            (EventDispatchers|BindEventtoOnSelected _returnvalue_2 (delegate Custom|OnSelected)))
          (:4
            (goto _label_2))
          (:5
            (Default|SetState _returnvalue_2 "NewEnumerator0" false :!label _label_3)
            (EventDispatchers|BindEventtoOnSelected _returnvalue_2 (delegate Custom|OnSelected)))
          (:6
            (goto _label_3))
          (:7
            (goto _label_3)))
        (else
          (bind _returnvalue_3 (Game|SpawnActorfromClass "/Game/Blueprints/BoardTile/BoardTileNull.BoardTileNull_C" (Math|Transform|MakeRelativeTransform (Math|Conversions|ToTransform(Vector) (Math|Vector|MakeVector _coordinate _coordinate_2 0.0)) (Transformation|GetActorTransform)) "Undefined" 0 0))
          (Default|SetTileColor _returnvalue_3 "NewEnumerator1")))))
  ;[1 1 1] Assign Tile Adjacencies
  (bind _result (Utilities|Set|ToArray (Variables|Default|GetTiles)))
  (for _array_element _result
    (Default|FindAdjacenciesfromSet _array_element _result)))

(fn ConstructionScript)

(fn TileIndextoCoordinate
  (params (Index :type Integer))
  (return (Math|Conversions|ToFloat(Integer) (- (* (- Index 3) 100) (/ (Variables|Default|GetTileSize) 2)))))

(fn EndPlayerTurn
  (if (Variables|Default|GetGameOver)
    (return)
    (else
      (switch Utilities|FlowControl|Switch|SwitchonETeamColor (Variables|Default|GetActivePlayer)
        (:NewEnumerator0
          (Variables|Default|SetActivePlayer "NewEnumerator1")
          (Variables|Default|SetbIsAITurn false))
        (:NewEnumerator1
          (Variables|Default|SetActivePlayer "NewEnumerator0")))
      (bind _hasmoves (CallFunction|PlayerHasMoves (Variables|Default|GetActivePlayer)))
      (CallFunction|ChangeHudText)
      (if _hasmoves
        (if (Utilities|Enum|Equal(Enum) (Variables|Default|GetActivePlayer) "NewEnumerator0")
          (CallFunction|CheckforWinner)
          (if (Variables|Default|GetGameOver)
            (return)
            (else
              (CallFunction|StartAITurn))))
        (else
          (Development|PrintString (Utilities|String|Append (Utilities|String|EnumtoString (Variables|Default|GetActivePlayer)) "HAS LOST!!?$") true true "(R=0.078899,G=0.833333,B=0.000000,A=1.000000)" 5.0)
          (if (Utilities|Enum|Equal(Enum) "Black" (Utilities|String|EnumtoString (Variables|Default|GetActivePlayer)))
            (bind _output_get (Variables|Default|SetPlayerWon true)))
          (CallFunction|ShowVictoryDefeatWidget _output_get))))))

(fn TileShouldKing
  (params (NewTile :type Board%20Tile%20Object%20Reference) (CurrentSelected :type Board%20Tile%20Object%20Reference))
  (bind _kinged (Variables|/Game/Blueprints/BoardTile/BoardTile.BoardTile_C|GetKinged CurrentSelected))
  (bind _row (Variables|/Game/Blueprints/BoardTile/BoardTile.BoardTile_C|GetRow NewTile))
  (bind _activeplayer (Variables|Default|GetActivePlayer))
  (if _kinged
    (Development|PrintString "Curr is Kinged"))
  (return (Math|Boolean|ORBoolean _kinged (and (== _row 0) (Utilities|Enum|Equal(Enum) _activeplayer "NewEnumerator0")) (and (== _row 7) (Utilities|Enum|Equal(Enum) _activeplayer "NewEnumerator1")))))

(fn PlayerHasMoves
  (params (Player :type ETeamColor%20Enum :default "NewEnumerator2"))
  (bind _result (Utilities|Set|ToArray (Variables|Default|GetTiles)))
  (for _array_element _result
    (if (Utilities|Enum|Equal(Enum) (Variables|/Game/Blueprints/BoardTile/BoardTile.BoardTile_C|GetState _array_element) Player)
      (bind _moves (Default|GetValidMoves _array_element false))
      (if (> (Utilities|Map|Length _moves) 0)
        (return true))))
  (return false))

(fn RunAITurn
  (bind _boardstate (CallFunction|MakeBoardState))
  (bind _output_get (LocalVariables|SetCurrentState _boardstate))
  (bind _movestruct (CallFunction|PickBestMove _output_get))
  (Default|Select (.FromTile (Utilities|Struct|BreakMoveStruct _movestruct)))
  (Default|Select (.ToTile (Utilities|Struct|BreakMoveStruct _movestruct)))
  (if (Variables|Default|GetForcedDoubleJump)
    (CallFunction|AIContinueForcedJump)))

(fn GetAllBlackMoves
  (Utilities|Array|Clear (LocalVariables|GetAllMoves))
  (bind _result (Utilities|Set|ToArray (Variables|Default|GetTiles)))
  (for _array_element _result
    (if (Utilities|Enum|Equal(Enum) (Variables|/Game/Blueprints/BoardTile/BoardTile.BoardTile_C|GetState _array_element) "NewEnumerator0")
      (bind _moves (Default|GetValidMoves _array_element false))
      (bind _keys (Utilities|Map|Keys _moves))
      (for _array_element_2 _keys
        (Utilities|Array|Add (LocalVariables|GetAllMoves) (Utilities|Struct|MakeMoveStruct _array_element _array_element_2))
        (Development|PrintString "From Tile:" false)
        (Development|PrintString (Utilities|GetDisplayName (.FromTile (Utilities|Struct|BreakMoveStruct (Utilities|Struct|MakeMoveStruct _array_element _array_element_2)))) false)
        (Development|PrintString "To Tile:" false)
        (Development|PrintString (Utilities|GetDisplayName (.ToTile (Utilities|Struct|BreakMoveStruct (Utilities|Struct|MakeMoveStruct _array_element _array_element_2)))) false))))
  (return (LocalVariables|GetAllMoves)))

(fn MakeBoardState
  (bind _result (Utilities|Set|ToArray (Variables|Default|GetTiles)))
  (for _array_element _result
    (switch Utilities|FlowControl|Switch|SwitchonETeamColor (Variables|/Game/Blueprints/BoardTile/BoardTile.BoardTile_C|GetState _array_element)
      (:NewEnumerator2
        (bind _output_get (LocalVariables|SetCode 0))
        (Utilities|Array|Add (LocalVariables|GetTileCodes) _output_get))
      (:NewEnumerator0
        (if (Variables|/Game/Blueprints/BoardTile/BoardTile.BoardTile_C|GetKinged _array_element)
          (bind _output_get_2 (LocalVariables|SetCode 4))
          (Utilities|Array|Add (LocalVariables|GetTileCodes) _output_get_2)
          (else
            (bind _output_get_3 (LocalVariables|SetCode 3))
            (Utilities|Array|Add (LocalVariables|GetTileCodes) _output_get_3))))
      (:NewEnumerator1
        (if (Variables|/Game/Blueprints/BoardTile/BoardTile.BoardTile_C|GetKinged _array_element)
          (bind _output_get_4 (LocalVariables|SetCode 2))
          (Utilities|Array|Add (LocalVariables|GetTileCodes) _output_get_4)
          (else
            (bind _output_get_5 (LocalVariables|SetCode 1))
            (Utilities|Array|Add (LocalVariables|GetTileCodes) _output_get_5))))))
  (return (Utilities|Struct|MakeBoardState (LocalVariables|GetTileCodes) (Variables|Default|GetActivePlayer))))

(fn EvaluateBoardState
  (params (BoardState :type Board%20State%20Structure))
  (LocalVariables|SetWhitePieces 0)
  (LocalVariables|SetBlackPieces 0)
  (for _array_element (.Tiles (Utilities|Struct|BreakBoardState BoardState))
    (switch int _array_element
      (:1
        (LocalVariables|Setthescore (+ (LocalVariables|Getthescore) -3.0))
        (LocalVariables|SetWhitePieces (+ (LocalVariables|GetWhitePieces) 1)))
      (:2
        (LocalVariables|Setthescore (+ (LocalVariables|Getthescore) -5.0))
        (LocalVariables|SetWhitePieces (+ (LocalVariables|GetWhitePieces) 1)))
      (:3
        (LocalVariables|Setthescore (+ (LocalVariables|Getthescore) 3.0))
        (LocalVariables|SetBlackPieces (+ (LocalVariables|GetBlackPieces) 1)))
      (:4
        (LocalVariables|Setthescore (+ (LocalVariables|Getthescore) 5.0))
        (LocalVariables|SetBlackPieces (+ (LocalVariables|GetBlackPieces) 1)))))
  (if (or (== (LocalVariables|GetWhitePieces) 0) (== (LocalVariables|GetBlackPieces) 0))
    (if (== (LocalVariables|GetBlackPieces) 0)
      (LocalVariables|Setthescore -1e+05)
      (else
        (LocalVariables|Setthescore 1e+05))))
  (return (LocalVariables|Getthescore)))

(fn ApplyMove
  (params (BoardState :type Board%20State%20Structure) (MoveStruct :type Move%20Struct%20Structure))
  (bind (_tiles _activeteam) (Utilities|Struct|BreakBoardState BoardState))
  (bind (_fromtile _totile) (Utilities|Struct|BreakMoveStruct MoveStruct))
  (LocalVariables|SetTilesCopy _tiles)
  (bind _result (Utilities|Set|ToArray (Variables|Default|GetTiles)))
  (LocalVariables|SetFromIndex (Utilities|Array|FindItem _result _fromtile))
  (LocalVariables|SetToIndex (Utilities|Array|FindItem _result _totile))
  (LocalVariables|SetPieceCode (Utilities|Array|Get(acopy) (LocalVariables|GetTilesCopy) (LocalVariables|GetFromIndex)))
  (Utilities|Array|SetArrayElem (LocalVariables|GetTilesCopy) (LocalVariables|GetFromIndex) 0)
  (Utilities|Array|SetArrayElem (LocalVariables|GetTilesCopy) (LocalVariables|GetToIndex) (LocalVariables|GetPieceCode))
  (if (Utilities|Enum|Equal(Enum) _activeteam "NewEnumerator1")
    (bind _output_get (LocalVariables|SetNextTeam "NewEnumerator0"))
    (return (Utilities|Struct|MakeBoardState (LocalVariables|GetTilesCopy) _output_get))
    (else
      (bind _output_get_2 (LocalVariables|SetNextTeam "NewEnumerator1"))
      (return (Utilities|Struct|MakeBoardState (LocalVariables|GetTilesCopy) _output_get_2)))))

(fn SimulateRandomMove
  (params (BoardState :type Board%20State%20Structure))
  (bind _output_get (LocalVariables|SetSimState BoardState))
  (while (< (LocalVariables|GetLoopCounter) 200)
    (switch Utilities|FlowControl|Switch|SwitchonETeamColor (.ActiveTeam (Utilities|Struct|BreakBoardState _output_get))
      (:NewEnumerator0
        (bind _newparam (CallFunction|GetAllBlackMoves))
        (LocalVariables|SetAvailableMoves _newparam))
      (:NewEnumerator1
        (bind _newparam_2 (CallFunction|GetAllWhiteMoves))
        (LocalVariables|SetAvailableMoves _newparam_2)))
    (if (> (Utilities|Array|Length (LocalVariables|GetAvailableMoves)) 0)
      (bind _board_state (CallFunction|ApplyMove (LocalVariables|GetSimState) (Utilities|Array|Get(acopy) (LocalVariables|GetAvailableMoves) (Math|Random|RandomIntegerinRange 0 (- (Utilities|Array|Length (LocalVariables|GetAvailableMoves)) 1)))))
      (bind _output_get_2 (LocalVariables|SetSimState _board_state))
      (bind _score (CallFunction|EvaluateBoardState _output_get_2))
      (return _score)
      (else
        (bind _score_2 (CallFunction|EvaluateBoardState _output_get))
        (return _score_2)))))

(fn GetAllWhiteMoves
  (Utilities|Array|Clear (LocalVariables|GetAllMoves))
  (bind _result (Utilities|Set|ToArray (Variables|Default|GetTiles)))
  (for _array_element _result
    (if (Utilities|Enum|Equal(Enum) (Variables|/Game/Blueprints/BoardTile/BoardTile.BoardTile_C|GetState _array_element) "NewEnumerator1")
      (bind _moves (Default|GetValidMoves _array_element false))
      (bind _keys (Utilities|Map|Keys _moves))
      (for _array_element_2 _keys
        (Utilities|Array|Add (LocalVariables|GetAllMoves) (Utilities|Struct|MakeMoveStruct _array_element _array_element_2))
        (Development|PrintString "From Tile:" false)
        (Development|PrintString (Utilities|GetDisplayName (.FromTile (Utilities|Struct|BreakMoveStruct (Utilities|Struct|MakeMoveStruct _array_element _array_element_2)))) false)
        (Development|PrintString "To Tile:" false)
        (Development|PrintString (Utilities|GetDisplayName (.ToTile (Utilities|Struct|BreakMoveStruct (Utilities|Struct|MakeMoveStruct _array_element _array_element_2)))) false))))
  (return (LocalVariables|GetAllMoves)))

(fn PickBestMove
  (params (BoardState :type Board%20State%20Structure))
  (bind _newparam (CallFunction|GetAllBlackMoves))
  (bind _output_get (LocalVariables|SetAvailableMoves _newparam))
  (LocalVariables|SetBestScore -1e+05)
  (for _array_element _output_get
    (bind _board_state (CallFunction|ApplyMove BoardState _array_element))
    (bind _output_get_2 (LocalVariables|SetSimState _board_state))
    (bind _resultscore (CallFunction|SimulateRandomMove _output_get_2))
    (if (> _resultscore (LocalVariables|GetBestScore))
      (LocalVariables|SetBestScore _resultscore)
      (LocalVariables|SetBestMove _array_element)))
  (return (LocalVariables|GetBestMove)))

(fn CheckforWinner
  (bind _hasmoves (CallFunction|PlayerHasMoves "NewEnumerator1"))
  (LocalVariables|SetWhiteHasMoves _hasmoves)
  (bind _hasmoves_2 (CallFunction|PlayerHasMoves "NewEnumerator0"))
  (LocalVariables|SetBlackHasMoves _hasmoves_2)
  (if (and (not (LocalVariables|GetWhiteHasMoves)) (not (LocalVariables|GetBlackHasMoves)))
    (Variables|Default|SetWinnerText "DRAW NO MOVES LEFT EITHER SIDE")
    (CallFunction|EndGame)
    (else
      (switch Utilities|FlowControl|Switch|SwitchonETeamColor (Variables|Default|GetActivePlayer)
        (:NewEnumerator0
          (if (not (LocalVariables|GetBlackHasMoves))
            (Variables|Default|SetPlayerWon true)
            (Variables|Default|SetWinnerText "White wins - Black has no legal moves")
            (CallFunction|EndGame)
            (else
              (return))))
        (:NewEnumerator1
          (if (not (LocalVariables|GetWhiteHasMoves))
            (Variables|Default|SetWinnerText "Black wins - White has no legal moves")
            (CallFunction|EndGame)
            (else
              (return))))))))

(fn ChangeHudText
  (bind _asnew_hud1 (Utilities|Casting|CastToNewHUD1 (HUD|GetHUD (Game|GetPlayerController 0))))
  (Default|ChangeText (Variables|/Game/Blueprints/NewHUD1.NewHUD1_C|GetUI_ref _asnew_hud1)))

(fn ShowVictoryDefeatWidget
  (params (Win/Lose :type Boolean))
  (Viewport|RemoveAllWidgets)
  (bind _returnvalue (UserInterface|CreateWidget "/Game/UI/W_VictoryDefeat.W_VictoryDefeat_C"))
  (bind _output_get (Variables|Default|SetVictoryDefeatWidget _returnvalue))
  (if Win/Lose
    _
    (else
      (Default|Lose _output_get)))
  (UserInterface|Viewport|AddtoViewport _output_get 0))