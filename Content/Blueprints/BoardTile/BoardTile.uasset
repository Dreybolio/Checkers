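; BoardTile is a checkers square actor that shows its piece, king icon and highlight, and broadcasts selection when clicked on White's turn.
; It finds the BoardManager on construction and clears its highlight whenever the manager signals a tile selection.
; It caches four diagonal neighbors from a tile set.
; Move and hop queries walk these links by color and kinged status, returning destination-to-captured-tile maps and optionally highlighting destinations.
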(event OnTileSelected(Manager)
  (params (Tile :type Board%20Tile%20Object%20Reference))
  (CallFunction|SetHighlighted false))

(event MouseInput|EventActorOnClicked
  (params (ButtonPressed :type Key%20Structure :default "None"))
  (if (Utilities|Enum|Equal(Enum) (Variables|/Game/Blueprints/BoardTile/BoardManager.BoardManager_C|GetActivePlayer (Variables|Default|GetManager)) "NewEnumerator1")
    (CallFunction|Select)))

(fn ConstructionScript
  (CallFunction|SetState (Variables|Default|GetState) (Variables|Default|GetKinged))
  (CallFunction|SetHighlighted (Variables|Default|GetHighlighted))
  (bind _returnvalue (Actor|GetActorOfClass "/Game/Blueprints/BoardTile/BoardManager.BoardManager_C"))
  (if (not (== _returnvalue 0))
    (Variables|Default|SetManager _returnvalue)))

(fn SetState
  (params (NewState :type ETeamColor%20Enum :default "NewEnumerator2") (Kinged :type Boolean))
  (bind _piece (Variables|Default|GetPiece))
  (bind _output_get (Variables|Default|SetKinged Kinged))
  (if Kinged
    (Development|PrintString "Set Kinged!"))
  (Rendering|SetVisibility (Variables|Default|GetKingIcon) _output_get true)
  (bind _output_get_2 (Variables|Default|SetState NewState))
  (switch Utilities|FlowControl|Switch|SwitchonETeamColor _output_get_2
    (:NewEnumerator2
      (Rendering|SetVisibility _piece false true))
    (:NewEnumerator0
      (Rendering|Material|SetMaterial _piece 0 "/Game/Materials/PieceBlack.PieceBlack")
      (Rendering|SetVisibility _piece true true :!label _label))
    (:NewEnumerator1
      (Rendering|Material|SetMaterial _piece 0 "/Game/Materials/PieceWhite.PieceWhite")
      (goto _label))))

(fn SetTileColor
  (params (Color :type ETeamColor%20Enum :default "NewEnumerator2"))
  (bind _staticmeshcomponent (Variables|Debug|GetStaticMeshComponent))
  (switch Utilities|FlowControl|Switch|SwitchonETeamColor Color
    (:NewEnumerator0
      (Rendering|Material|SetMaterial _staticmeshcomponent 0 "/Game/Materials/TileBlack.TileBlack"))
    (:NewEnumerator1
      (Rendering|Material|SetMaterial _staticmeshcomponent 0 "/Game/Materials/TileWhite.TileWhite"))))

(fn Select
  (Default|CallOnSelected self))

(fn SetHighlighted
  (params (Highlighted :type Boolean))
  (bind _output_get (Variables|Default|SetHighlighted Highlighted))
  (Rendering|SetVisibility (Variables|Default|GetHighlight) _output_get false)
  (if _output_get
    _))

(fn FindAdjacenciesfromSet
  (params (Tiles :type Array%20of%20Board%20Tile%20Object%20References))
  (bind _row (Variables|Default|GetRow))
  (bind _column (Variables|Default|GetColumn))
  (bind _array_element (Utilities|Array|ForEachLoopwithBreak Tiles :!label _label)
    (:LoopBody
      (if (and (== (Variables|BoardTile_C|GetRow _array_element) (- _row 1)) (== (Variables|BoardTile_C|GetColumn _array_element) (- _column 1)))
        (Variables|Default|SetTileBwdL _array_element)
        (if (Math|Boolean|ANDBoolean (!= (Variables|Default|GetTileFwdL) 0) (!= (Variables|Default|GetTileFwdR) 0) (!= (Variables|Default|GetTileBwdL) 0) (!= (Variables|Default|GetTileBwdR) 0)) :!label _label_2
          (goto _label Break))
        (elif (and (== (Variables|BoardTile_C|GetRow _array_element) (- _row 1)) (== (Variables|BoardTile_C|GetColumn _array_element) (+ _column 1)))
          (Variables|Default|SetTileBwdR _array_element)
          (goto _label_2)
          (elif (and (== (Variables|BoardTile_C|GetRow _array_element) (+ _row 1)) (== (Variables|BoardTile_C|GetColumn _array_element) (- _column 1)))
            (Variables|Default|SetTileFwdL _array_element)
            (goto _label_2)
            (elif (and (== (Variables|BoardTile_C|GetRow _array_element) (+ _row 1)) (== (Variables|BoardTile_C|GetColumn _array_element) (+ _column 1)))
              (Variables|Default|SetTileFwdR _array_element)
              (goto _label_2))))))))

(fn GetValidMoves
  (params (DoHighlight :type Boolean))
  (bind _foundmoves (LocalVariables|GetFoundMoves))
  (bind _kinged (Variables|Default|GetKinged))
  (bind _state (Variables|Default|GetState))
  (bind _kinged_2 (Variables|Default|GetKinged))
  (bind _state_2 (Variables|Default|GetState))
  (bind _returnvalue (Utilities|Enum|Equal(Enum) _state "NewEnumerator0"))
  (bind _returnvalue_2 (Utilities|Enum|Equal(Enum) _state_2 "NewEnumerator1"))
  (bind _returnvalue_3 (or _kinged _returnvalue))
  (bind _returnvalue_4 (or _kinged_2 _returnvalue_2))
  (if _returnvalue_4
    (bind (_destination _eliminate) (CallFunction|CheckDirectionforMoves "NewEnumerator2" DoHighlight))
    (if (!= _destination 0)
      (Utilities|Map|Add _foundmoves _destination _eliminate)))
  (if _returnvalue_4
    (bind (_destination_2 _eliminate_2) (CallFunction|CheckDirectionforMoves "NewEnumerator0" DoHighlight))
    (if (!= _destination_2 0)
      (Utilities|Map|Add _foundmoves _destination_2 _eliminate_2)))
  (if _returnvalue_3
    (bind (_destination_3 _eliminate_3) (CallFunction|CheckDirectionforMoves "NewEnumerator1" DoHighlight))
    (if (!= _destination_3 0)
      (Utilities|Map|Add _foundmoves _destination_3 _eliminate_3)))
  (if _returnvalue_3
    (bind (_destination_4 _eliminate_4) (CallFunction|CheckDirectionforMoves "NewEnumerator3" DoHighlight))
    (if (!= _destination_4 0)
      (Utilities|Map|Add _foundmoves _destination_4 _eliminate_4)))
  (return _foundmoves))

(fn GetValidHops
  (params (DoHighlight :type Boolean))
  (bind _foundmoves (LocalVariables|GetFoundMoves))
  (bind _kinged (Variables|Default|GetKinged))
  (bind _state (Variables|Default|GetState))
  (bind _kinged_2 (Variables|Default|GetKinged))
  (bind _state_2 (Variables|Default|GetState))
  (bind _returnvalue (Utilities|Enum|Equal(Enum) _state "NewEnumerator0"))
  (bind _returnvalue_2 (Utilities|Enum|Equal(Enum) _state_2 "NewEnumerator1"))
  (bind _returnvalue_3 (or _kinged _returnvalue))
  (bind _returnvalue_4 (or _kinged_2 _returnvalue_2))
  (if _returnvalue_4
    (bind (_destination _eliminate) (CallFunction|CheckDirectionforMoves "NewEnumerator2" DoHighlight))
    (if (!= _eliminate 0)
      (Utilities|Map|Add _foundmoves _destination _eliminate)))
  (if _returnvalue_4
    (bind (_destination_2 _eliminate_2) (CallFunction|CheckDirectionforMoves "NewEnumerator0" DoHighlight))
    (if (!= _eliminate_2 0)
      (Utilities|Map|Add _foundmoves _destination_2 _eliminate_2)))
  (if _returnvalue_3
    (bind (_destination_3 _eliminate_3) (CallFunction|CheckDirectionforMoves "NewEnumerator1" DoHighlight))
    (if (!= _eliminate_3 0)
      (Utilities|Map|Add _foundmoves _destination_3 _eliminate_3)))
  (if _returnvalue_3
    (bind (_destination_4 _eliminate_4) (CallFunction|CheckDirectionforMoves "NewEnumerator3" DoHighlight))
    (if (!= _eliminate_4 0)
      (Utilities|Map|Add _foundmoves _destination_4 _eliminate_4)))
  (return _foundmoves))

(fn CheckDirectionforMoves
  (params (Direction :type EDirection%20Enum :default "NewEnumerator2") (DoHightlight :type Boolean))
  (bind _tile (CallFunction|GetTileinDirection Direction))
  (if (!= _tile 0)
    (if (Utilities|Enum|Equal(Enum) (Variables|BoardTile_C|GetState _tile) "NewEnumerator2")
      (CallFunction|SetHighlighted _tile DoHightlight)
      (return _tile 0)
      (else
        (bind _tile_2 (CallFunction|GetTileinDirection _tile Direction))
        (if (!= _tile_2 0)
          (if (and (Utilities|Enum|NotEqual(Enum) (Variables|BoardTile_C|GetState _tile) (Variables|Default|GetState)) (Utilities|Enum|Equal(Enum) (Variables|BoardTile_C|GetState _tile_2) "NewEnumerator2"))
            (CallFunction|SetHighlighted _tile_2 DoHightlight)
            (return _tile_2 _tile)
            (else
              _))))))
  (return 0 0))

(fn GetTileinDirection
  (params (Direction :type EDirection%20Enum :default "NewEnumerator2"))
  (switch Utilities|FlowControl|Switch|SwitchonEDirection Direction
    (:NewEnumerator2
      (return (Variables|Default|GetTileFwdL)))
    (:NewEnumerator0
      (return (Variables|Default|GetTileFwdR)))
    (:NewEnumerator1
      (return (Variables|Default|GetTileBwdL)))
    (:NewEnumerator3
      (return (Variables|Default|GetTileBwdR)))))